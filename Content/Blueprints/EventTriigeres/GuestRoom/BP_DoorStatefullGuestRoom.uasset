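; Sliding guest room door actor that opens or closes according to the condition passed to SetActivationState.
; A timeline plays forward to open and reverses to close, offsetting the door along its right vector from the location cached at BeginPlay.
; Each state change prints a debug string, and the interaction anchor and type functions return only zero and None.
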(event EventBeginPlay
  (Variables|Default|SetStartLocation (Transformation|GetActorLocation)))

(event EventSetActivationState
  (params (bConditionMet :type Boolean) (Activator :type Actor%20Object%20Reference))
  (if bConditionMet
    (Development|PrintString "DoorOpen")
    (bind _movedoory (Timeline|タイムライン Play)
      (:Update
        (Transformation|SetActorLocation (+ (Variables|Default|GetStartLocation) (* _movedoory (Transformation|GetActorRightVector))) false false)))
    (else
      (Development|PrintString "DoorClose")
      (Timeline|タイムライン Reverse))))

(fn ConstructionScript)

(fn GetInteractionAnchorLocation
  (return "0, 0, 0"))

(fn GetInteractionType
  (return "None"))