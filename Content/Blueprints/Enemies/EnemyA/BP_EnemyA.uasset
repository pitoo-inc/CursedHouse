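; BP_EnemyA is an enemy actor that takes point damage, staggers and dies through its HitReaction component.
; Point damage passes to HitReaction with the hit physical material and direction for per-part damage, and is also reported to AI damage sensing.
; HitReaction's stagger event plays the StaggerData montage.
; Its death event plays a dying montage and destroys the actor on blend out, with debug prints on both events.
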(event OnStaggerTriggered(HitReaction)
  (params (StaggerData :type Stagger%20Data%20Structure) (HitDirection :type Vector :default "0, 0, 0") (HitPhysMat :type Physical%20Material%20Object%20Reference))
  (Development|PrintString (Utilities|GetDisplayName HitPhysMat))
  (Animation|Montage|PlayMontage (Variables|Character|GetMesh) (.staggermontage StaggerData)))

(event OnDeath(HitReaction)
  (Development|PrintString "死亡")
  (Animation|Montage|PlayMontage (Variables|Character|GetMesh) "/HitReaction/Sample/Mixamo/ReTarget/Anims/AnimationMontages/AM_HR_Dying.AM_HR_Dying"
    (:OnBlendOut
      (Actor|DestroyActor))))

(event Game|Damage|EventPointDamage
  (params (Damage :type Float%20%28single-precision%29) (DamageType :type Damage%20Type%20Object%20Reference) (HitLocation :type Vector :default "0, 0, 0") (HitNormal :type Vector :default "0, 0, 0") (HitComponent :type Primitive%20Component%20Object%20Reference) (BoneName :type Name :default "None") (ShotFromDirection :type Vector :default "0, 0, 0") (InstigatedBy :type Controller%20Object%20Reference) (DamageCauser :type Actor%20Object%20Reference) (HitInfo :type Hit%20Result%20Structure%20%28by%20ref%29))
  (Class|HitReactionComponent|ApplyPartDamage (Variables|Default|GetHitReaction) Damage (.PhysMat (Collision|BreakHitResult HitInfo)) ShotFromDirection DamageCauser)
  (Class|AISenseDamage|ReportDamageEvent self DamageCauser Damage (Transformation|GetActorLocation DamageCauser) HitLocation "None"))

(fn ConstructionScript)