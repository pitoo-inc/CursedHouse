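; BP_TriggerA is an interactable trigger, styled as a card reader, that notifies its ConditionSource to drive something like a door.
; OnInteract locks interaction, activates the condition and rescales the reader identically for either toggle state.
; One-shot mode disables the proximity sensor's collision; otherwise, after five seconds it reactivates the condition, to close the door, and unlocks.
; A "KeyA" inventory check exists but is disconnected.
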(event EventOnInteract
  (params (InstigatorActor :type Actor%20Object%20Reference))
  (bind _cardreader (Variables|Default|GetCardReader))
  (if (Variables|Default|GetbCanInteract)
    ;[0.15 0.15 0.15 0.5] インターラクトできないようにした後にActibateに通知
    (Variables|Default|SetbCanInteract false)
    (Class|ConditionSourceComponent|ActivateCondition (Variables|Default|GetConditionSource))
    (bind _output_get (Variables|Default|SetbIsToggled (not (Variables|Default|GetbIsToggled))))
    ;[1 1 0 0.5] 独自処理：IsToggledでカードリーダの読み込みを表現
    (if _output_get
      (Transformation|SetRelativeScale3D _cardreader "0.100000,0.500000,0.500000")
      (else
        (Transformation|SetRelativeScale3D _cardreader "0.100000,0.500000,0.500000")))
    (if (Variables|Default|GetbIsOneShot)
      ;[0.15 0.15 0.15 0.5] 一回だけ実行の場合はインターラクトのセンサー用のコリジョン機能をＯＦＦ
      (Collision|SetCollisionEnabled (Variables|Default|GetProximitySensor) "NoCollision")
      (else
        ;[1 1 0 0.5] 独自処理：5秒後後にインターラクトを再開。ドアを閉めたいのでActibateに通知
        (Utilities|FlowControl|Delay 5.0)
        (Class|ConditionSourceComponent|ActivateCondition (Variables|Default|GetConditionSource))
        (Variables|Default|SetbCanInteract true)))))

(fn ConstructionScript)