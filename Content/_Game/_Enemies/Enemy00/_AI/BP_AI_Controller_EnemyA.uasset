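; AI controller for EnemyA that runs its behavior tree on BeginPlay and feeds it perception results through the blackboard.
; Seeing the player sets TargetActor; losing sight clears it and stores the player's current position as InvestigateLocation.
; Successfully sensed hearing or damage stimuli write their source location to InvestigateLocation.
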(event OnTargetPerceptionUpdated(AIPerception)
  (params (Actor :type Actor%20Object%20Reference) (Stimulus :type AI%20Stimulus%20Structure))
  (bind (_age _expirationage _strength _stimuluslocation _receiverlocation _tag _bsuccessfullysensed) (Utilities|Struct|BreakAIStimulus Stimulus))
  (bind _returnvalue (AI|GetBlackboard 0))
  ;[0.15 0.15 0.15 0.5] センサー枚に反応した呼ばれる
  (bind _returnvalue_2 (Class|AIPerceptionSystem|GetSenseClassforStimulus Stimulus))
  ;[0.15 0.15 0.15 0.5] プレイヤーが視覚に入った、見失った
  (if (== _returnvalue_2 "/Script/AIModule.AISense_Sight")
    (if (== Actor (Game|Player|GetPlayerPawn 0))
      (if _bsuccessfullysensed
        ;;[0.15 0.15 0.15 0.5] 視覚内に入ったら
        (Development|PrintString "視覚内")
        (AI|Components|Blackboard|SetValueasObject (AI|GetBlackboard 0) (Utilities|Name|MakeLiteralName "TargetActor") Actor)
        (else
          ;;[0.15 0.15 0.15 0.5] 見失ったら、最後に見たプレイヤーの位置を警戒
          (Development|PrintString "視覚外")
          (AI|Components|Blackboard|SetValueasObject _returnvalue (Utilities|Name|MakeLiteralName "TargetActor") 0)
          (AI|Components|Blackboard|SetValueasVector _returnvalue (Utilities|Name|MakeLiteralName "InvestigateLocation") (Transformation|GetActorLocation (Game|Player|GetPlayerPawn 0))))))
    (else
      ;[0.15 0.15 0.15 0.5] 聴覚 or 攻撃されたら、発生源の位置まで移動してを警戒
      (if (or (== _returnvalue_2 "/Script/AIModule.AISense_Hearing") (== _returnvalue_2 "/Script/AIModule.AISense_Damage"))
        (if _bsuccessfullysensed
          (AI|Components|Blackboard|SetValueasVector (AI|GetBlackboard 0) (Utilities|Name|MakeLiteralName "InvestigateLocation") _stimuluslocation))))))

(event EventBeginPlay
  (AI|RunBehaviorTree "/Game/_Game/_Enemies/Enemy00/_AI/BT_AI_EnemyA.BT_AI_EnemyA"))

(fn ConstructionScript)