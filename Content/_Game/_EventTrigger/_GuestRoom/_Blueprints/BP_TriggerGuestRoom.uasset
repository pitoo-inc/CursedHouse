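; Interactable guest room trigger that fires only when the instigator's inventory component holds the guest room key.
; On success it locks interaction, activates its ConditionSource and flips its toggled state.
; One-shot triggers then disable proximity sensor collision, while repeatable ones re-enable interaction after a 2-second delay, though the inline comment says five.
; Without the key, it prints a Japanese message saying a key seems to be needed.
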(event EventOnInteract
  (params (InstigatorActor :type Actor%20Object%20Reference))
  (if (Variables|Default|GetbCanInteract)
    ;[1 1 0 0.5] 独自処理：インターラクトできるための条件
    (if (Class|RSInventoryComponent|HasItem (Actor|GetComponentbyClass InstigatorActor "/Script/EventSystem.RSInventoryComponent") "KeyGuestRoom")
      ;[0.15 0.15 0.15 0.5] インターラクトできないようにした後にActibateに通知
      (Variables|Default|SetbCanInteract false)
      (Class|ConditionSourceComponent|ActivateCondition (Variables|Default|GetConditionSource))
      (Variables|Default|SetbIsToggled (not (Variables|Default|GetbIsToggled)))
      (if (Variables|Default|GetbIsOneShot)
        ;[0.15 0.15 0.15 0.5] 一回だけ実行の場合はインターラクトのセンサー用のコリジョン機能をＯＦＦ
        (Collision|SetCollisionEnabled (Variables|Default|GetProximitySensor) "NoCollision")
        (else
          ;[1 1 0 0.5] 独自処理：5秒後後にインターラクトを再開
          (Utilities|FlowControl|Delay 2.0)
          (Variables|Default|SetbCanInteract true)))
      (else
        (Development|PrintString "鍵がいるようだ")))))

(fn ConstructionScript)